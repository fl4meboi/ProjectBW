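; BP_OSC receives Alpha Absolute and Beta Absolute readings over OSC and stores them as float variables.
; On BeginPlay it starts a listening OSC server on a hardcoded IP and port and binds the message event.
; Each message is routed by the last segment of its address, and its first float updates AlphaValue or BetaValue.
; Disconnected leftovers include an alternate server, an address debug print and an accelerometer threshold test.
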(event `self.ReceiveBeginPlay`
  (bind _returnvalue (`OSCManager.CreateOSCServer` "192.168.137.1" 5000 false true "" null))
  (bind _output_get (set `self.OSCServer` _returnvalue))
  (add `OSCServer.OnOscMessageReceived` _output_get (`|CreateDelegate` :!event `OSCIn`)))

(event `OSCIn`
  (params (Message :type "OSCMessage Structure (by ref)") (IPAddress :type String) (Port :type Integer))
  (bind _output_get (set `self.OSCMessages` Message)) ; OSC 신호값 저장
  (bind _returnvalue (`OSCManager.GetOSCMessageAddress` _output_get))
  (bind _returnvalue_2 (`OSCManager.GetOSCAddressFullPath` _returnvalue)) ; OSC 신호값 텍스트(string)으로 변환
  (switch `string` (`.RightS` (`KismetStringLibrary.Split` _returnvalue_2 "/" "IgnoreCase" "FromEnd"))
    (:`alpha_absolute`
      ;[1 1 1] Alpha, Beta Value OSC 신호 받아서 set
      (bind _value (`OSCManager.GetFloat` (`self.OSCMessages`)))
      (set `self.AlphaValue` _value))
    (:`beta_absolute`
      (bind _value_2 (`OSCManager.GetFloat` (`self.OSCMessages`)))
      (set `self.BetaValue` _value_2))))

(fn `UserConstructionScript`)