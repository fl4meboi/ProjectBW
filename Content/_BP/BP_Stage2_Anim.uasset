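; Stage 2 actor that switches media playback according to an Alpha signal received through BP_OSC.
; BeginPlay finds the OSC actor and opens the first clip, then Tick reads its AlphaValue every frame.
; AlphaEmotionFunc sorts the value into three emotion steps and reports only changes, so the media is not restarted repeatedly.
; The third step opens Beta_02 rather than an Alpha clip; the visibility and skeletal mesh swap logic is disconnected.
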(event `self.ReceiveBeginPlay`
  ;[1 1 1] OSC 신호 가져오기
  (`self.EnableInput` (`GameplayStatics.GetPlayerController` 0))
  (bind _returnvalue (`GameplayStatics.GetActorOfClass` "/Game/_BP/BP_OSC.BP_OSC_C"))
  (set `self.BP_OSC` _returnvalue)
  ;[1 1 1] 처음 Media 재생해주기
  (`MediaPlayer.OpenSource` (`self.Media`) "/Game/Resources/Alpha_01.Alpha_01"))

(event `self.ReceiveTick`
  (params (DeltaSeconds :type "Float (single-precision)"))
  ;[1 1 1] Alpha Value print
  (set `self.Alpha Value` (`/Game/_BP/BP_OSC.AlphaValue` (`self.BP_OSC`)))
  (bind _bapplynewemotion (`self.AlphaEmotionFunc`))
  (if _bapplynewemotion
    ;[1 1 1] Emotion에서 Set한 각 단계에 따라Media change
    (switch `/Game/_BP/E_AlphaSteps` (`self.Emotion`)
      (:`NewEnumerator0`
        (`MediaPlayer.OpenSource` (`self.Media`) "/Game/Resources/Alpha_01.Alpha_01"))
      (:`NewEnumerator1`
        (`MediaPlayer.OpenSource` (`self.Media`) "/Game/Resources/Alpha_02.Alpha_02"))
      (:`NewEnumerator2`
        (`MediaPlayer.OpenSource` (`self.Media`) "/Game/Resources/Beta_02.Beta_02")))))

(event `ImpulseStage`)

(fn `AlphaEmotionFunc`
  (returns (bApplyNewEmotion :type Boolean))
  (set `self.OldEmotion` (`self.Emotion`))
  ;[1 1 1] 단계에 따른 animation play
  (if (<= (`self.Alpha Value`) 0.3)
    (set `self.Emotion` "NewEnumerator0")
    (elif (<= (`self.Alpha Value`) 1.0)
      (set `self.Emotion` "NewEnumerator1")
      (else
        (set `self.Emotion` "NewEnumerator2"))))
  ;[1 1 1] 같은 감정일 때는 반복적으로 글리치 재생되지 않도록
  (if (not (`|EnumEquality` (`self.Emotion`) (`self.OldEmotion`)))
    (return true)
    (else
      (return false))))

(fn `UserConstructionScript`)