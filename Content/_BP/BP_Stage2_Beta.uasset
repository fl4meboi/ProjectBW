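; Stage 2 actor that turns the Beta signal from BP_OSC into changes of video and skeletal mesh material.
; Each Tick it copies BetaValue, and BetaEmotionFunc sorts it into three emotion steps by threshold.
; Media and material switch only when the step changes, so playback is not restarted every frame.
; Alpha-driven logic, including visibility switching and an empty ImpulseStage event, remains but is not wired to run.
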(event `self.ReceiveBeginPlay`
  ;[1 1 1] OSC 신호 가져오기
  (`self.EnableInput` (`GameplayStatics.GetPlayerController` 0))
  (bind _returnvalue (`GameplayStatics.GetActorOfClass` "/Game/_BP/BP_OSC.BP_OSC_C"))
  (set `self.BP_OSC` _returnvalue)
  ;[1 1 1] 처음 Media 재생해주기
  (`MediaPlayer.OpenSource` (`self.Media`) "/Game/Resources/Beta_01.Beta_01"))

(event `self.ReceiveTick`
  (params (DeltaSeconds :type "Float (single-precision)"))
  (bind _betaemotion (`self.BetaEmotion`))
  ;[1 1 1] Alpha Value print
  (set `self.Beta Value` (`/Game/_BP/BP_OSC.BetaValue` (`self.BP_OSC`)))
  (bind _bapplynewemotion (`self.BetaEmotionFunc`))
  (if _bapplynewemotion
    ;[1 1 1] Emotion에서 Set한 각 단계에 따라Media change
    (switch `/Game/_BP/E_BetaSteps` (`self.BetaEmotion`)
      (:`NewEnumerator0`
        (`MediaPlayer.OpenSource` (`self.Media`) "/Game/Resources/Limbo.Limbo")
        (`PrimitiveComponent.SetMaterial` (`self.SkeletalMesh`) 0 "/Game/_MAT/NewCharacter_UV/BetaWhite_Mat.BetaWhite_Mat")
        (`KismetSystemLibrary.PrintString` (`|GetEnumeratorNameAsString` _betaemotion)))
      (:`NewEnumerator1`
        (`MediaPlayer.OpenSource` (`self.Media`) "/Game/Resources/Beta_01.Beta_01")
        (`PrimitiveComponent.SetMaterial` (`self.SkeletalMesh`) 0 "/Game/_MAT/NewCharacter_UV/Beta_Mat.Beta_Mat")
        (`KismetSystemLibrary.PrintString` (`|GetEnumeratorNameAsString` _betaemotion)))
      (:`NewEnumerator2`
        (`MediaPlayer.OpenSource` (`self.Media`) "/Game/Resources/Beta_02.Beta_02")
        (`PrimitiveComponent.SetMaterial` (`self.SkeletalMesh`) 0 "/Game/_MAT/NewCharacter_UV/BetaNavy_Mat.BetaNavy_Mat")
        (`KismetSystemLibrary.PrintString` (`|GetEnumeratorNameAsString` _betaemotion))))))

(event `ImpulseStage`)

(fn `AlphaEmotionFunc`
  (returns (bApplyNewEmotion :type Boolean))
  (set `self.AlphaOldEmotion` (`self.AlphaEmotion`))
  ;[1 1 1] 단계에 따른 animation play
  (if (<= (`self.Alpha Value`) 0.3)
    (set `self.AlphaEmotion` "NewEnumerator0")
    (elif (<= (`self.Alpha Value`) 1.0)
      (set `self.AlphaEmotion` "NewEnumerator1")
      (else
        (set `self.AlphaEmotion` "NewEnumerator2"))))
  ;[1 1 1] 같은 감정일 때는 반복적으로 글리치 재생되지 않도록
  (if (not (`|EnumEquality` (`self.AlphaEmotion`) (`self.AlphaOldEmotion`)))
    (return true)
    (else
      (return false))))

(fn `BetaEmotionFunc`
  (returns (bApplyNewEmotion :type Boolean))
  (set `self.BetaOldEmotion` (`self.BetaEmotion`))
  (if (<= (`self.Beta Value`) 0.4)
    (set `self.BetaEmotion` "NewEnumerator0")
    (elif (<= (`self.Beta Value`) 0.8)
      (set `self.BetaEmotion` "NewEnumerator1")
      (else
        (set `self.BetaEmotion` "NewEnumerator2"))))
  (if (not (`|EnumEquality` (`self.BetaEmotion`) (`self.BetaOldEmotion`)))
    (return true)
    (else
      (return false))))

(fn `UserConstructionScript`)