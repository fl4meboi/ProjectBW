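; BP_Stage1 is a stage actor that switches between six emotion versions of a visual (Angry, Worried, Surprised, Confused, Terrified, Happy) from a BPOSC value.
; Each Tick it prints and truncates BPOSC.AlphaValue, then hides the preceding version and shows the next in a fixed cycle.
; BeginPlay enables player input.
; The Emotion switch and ImpulseStage are empty, and the impulse and mesh-animation logic is disconnected.
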(event `CustomEvent`
  (switch `/Game/_BP/E_AlphaSteps` (`self.Emotion`)))

(event `self.ReceiveBeginPlay`
  (`self.EnableInput` (`GameplayStatics.GetPlayerController` 0)))

(event `self.ReceiveTick`
  (params (DeltaSeconds :type "Float (single-precision)"))
  (bind _alphavalue (`/Game/_BP/BP_OSC.AlphaValue` (`self.BP_OSC`)))
  (`KismetSystemLibrary.PrintString` (`KismetStringLibrary.Conv_DoubleToString` _alphavalue))
  (switch `int` (`KismetMathLibrary.FTrunc` _alphavalue)
    (:`0`
      (`SceneComponent.SetVisibility` (`self.Angry_ver2`) false false)
      (`SceneComponent.SetVisibility` (`self.Worried_ver2`) true false))
    (:`1`
      (`SceneComponent.SetVisibility` (`self.Worried_ver2`) false false)
      (`SceneComponent.SetVisibility` (`self.Surprised_ver2`) true false))
    (:`2`
      (`SceneComponent.SetVisibility` (`self.Surprised_ver2`) false false)
      (`SceneComponent.SetVisibility` (`self.Confused_ver2`) true false))
    (:`3`
      (`SceneComponent.SetVisibility` (`self.Confused_ver2`) false false)
      (`SceneComponent.SetVisibility` (`self.Terrified_ver2`) true false))
    (:`4`
      (`SceneComponent.SetVisibility` (`self.Terrified_ver2`) false false)
      (`SceneComponent.SetVisibility` (`self.Happy_ver2`) true false))
    (:`5`
      (`SceneComponent.SetVisibility` (`self.Happy_ver2`) false false)
      (`SceneComponent.SetVisibility` (`self.Angry_ver2`) true false))))

(event `ImpulseStage`)

(fn `UserConstructionScript`)